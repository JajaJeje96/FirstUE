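; ShipCar_BP is a player-controlled ship/car pawn with movement, mouse look and camera zoom.
; Vertical and horizontal axes add movement input along the actor's forward and right vectors, while mouse axes drive controller pitch and yaw.
; The Zoom axis adds a scaled offset to the SpringArm length, with no clamping.
; BeginPlay, Tick, overlap and the construction script are empty.
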(event `self.ReceiveTick`
  (params (DeltaSeconds :type "Float (single-precision)")))

(event `InputAxis|MoveVertical`
  (params (AxisValue :type "Float (single-precision)"))
  (`self.AddMovementInput` (`self.GetActorForwardVector`) AxisValue))

(event `InputAxis|MoveHorizontal`
  (params (AxisValue :type "Float (single-precision)"))
  (`self.AddMovementInput` (`self.GetActorRightVector`) AxisValue))

(event `InputAxis|Zoom`
  (params (AxisValue :type "Float (single-precision)"))
  (bind _springarm (`self.SpringArm`))
  (set `SpringArmComponent.TargetArmLength` (+ (* AxisValue 5.0) (`SpringArmComponent.TargetArmLength` _springarm)) _springarm))

(event `InputAxis|MouseHorintal`
  (params (AxisValue :type "Float (single-precision)"))
  (`self.AddControllerYawInput` AxisValue))

(event `InputAxis|MouseVertical`
  (params (AxisValue :type "Float (single-precision)"))
  (`self.AddControllerPitchInput` AxisValue))

(fn `UserConstructionScript`)