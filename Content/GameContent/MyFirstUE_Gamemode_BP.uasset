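; Game mode Blueprint that tracks how many cars are inside and decides when the player has won.
; Custom events AddCar and RemoveCar increment or decrement the current count, then share one check against the total needed to win.
; The check only prints a green Spanish win message or a red "not yet" message on screen.
; Nothing in this graph calls either event.
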(event `AddCar`
  (`/Engine/EditorBlueprintResources/StandardMacros.IncrementInt` (`self.CurrentCarsInside`)
    (:`  `
      (if (>= (`self.CurrentCarsInside`) (`self.TotalNumCarsToWin`)) :!label _label
        (`KismetSystemLibrary.PrintString` "Has ganado!" true true (struct :`R` 0.12946 :`G` 1.0 :`B` 0.109634 :`A` 1.0) 10.0)
        (else
          (`KismetSystemLibrary.PrintString` "Todavia no" true true (struct :`R` 1.0 :`G` 0.052083 :`B` 0.052083 :`A` 1.0)))))))

(event `RemoveCar`
  (`/Engine/EditorBlueprintResources/StandardMacros.DecrementInt` (`self.CurrentCarsInside`)
    (:`  `
      (goto _label))))

(fn `UserConstructionScript`)